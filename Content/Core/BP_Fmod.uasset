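; BP_Fmod drives in-game music through FMOD, reacting to low player health.
; On BeginPlay it starts the Mus_InGame event in 2D, stores the instance, and caches the GS_GGJ game state.
; Tick, throttled by a 0.2 second Delay, sets the music's GameState parameter to 1 when either player's HP drops below 6; nothing in this Blueprint resets it.
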(event EventBeginPlay
  (Utilities|FlowControl|Sequence
    (:then_0
      (bind _returnvalue (Class|FMODBlueprintStatics|PlayEvent2D "/Game/FMOD/Events/MUS/Mus_InGame.Mus_InGame"))
      (Variables|Default|SetBG%20music _returnvalue))
    (:then_1
      (bind _asgs_ggj (Utilities|Casting|CastToGS_GGJ (Game|GetGameState)))
      (Variables|Default|SetAs%20GS%20GGJ _asgs_ggj))))

(event EventTick
  (params (DeltaSeconds :type Float%20%28single-precision%29))
  (bind _as_gs_ggj (Variables|Default|GetAs%20GS%20GGJ))
  (Utilities|FlowControl|Delay 0.2)
  (if (or (< (Variables|/Game/Core/GS_GGJ.GS_GGJ_C|Getplayer1hp _as_gs_ggj) 6) (< (Variables|/Game/Core/GS_GGJ.GS_GGJ_C|Getplayer2hp _as_gs_ggj) 6))
    (Class|FMODBlueprintStatics|EventInstanceSetParameter (Variables|Default|GetBG%20music) "GameState" 1.0)))

(fn ConstructionScript)