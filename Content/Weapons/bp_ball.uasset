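; BP_Ball is a short-lived weapon projectile that damages players on contact and removes itself two seconds after spawning.
; The construction script gives the mesh a dynamic material instance of M_BULLET.
; When the sphere overlaps a player other than its owner, it swaps the material texture, applies damage, stops movement and is destroyed after a brief delay that leaves the new texture visible.
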(event OnComponentBeginOverlap(Sphere)
  (params (OverlappedComponent :type Primitive%20Component%20Object%20Reference) (OtherActor :type Actor%20Object%20Reference) (OtherComp :type Primitive%20Component%20Object%20Reference) (OtherBodyIndex :type Integer) (bFromSweep :type Boolean) (SweepResult :type Hit%20Result%20Structure%20%28by%20ref%29))
  (if (not (== OtherActor (Components|GetOwner)))
    (bind _asbp_player (Utilities|Casting|CastToBP_Player OtherActor))
    (Rendering|Material|SetTextureParameterValue (Variables|Default|GetDMI) "tex" "/Game/Weapons/T_BULLE2.T_BULLE2")
    (Game|Damage|ApplyDamage _asbp_player 1.0 0 0)
    (Components|Movement|StopMovementImmediately (Variables|Default|GetProjectileMovement))
    (Utilities|FlowControl|Delay 0.2)
    (Actor|DestroyActor)))

(event EventBeginPlay
  (Utilities|FlowControl|Delay 2.0)
  (Actor|DestroyActor))

(fn ConstructionScript
  (bind _staticmesh (Variables|Default|GetStaticMesh))
  (bind _returnvalue (Rendering|Material|CreateDynamicMaterialInstance _staticmesh 0 "/Game/Weapons/m_BULLET.m_BULLET" "None" :!class /Script/Engine.PrimitiveComponent))
  (bind _output_get (Variables|Default|SetDMI _returnvalue))
  (Rendering|Material|SetMaterial _staticmesh 0 _output_get))